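; VR motion controller actor for one hand that grabs physics props and shows a CPU readout.
; Grab picks the nearest simulating StaticMeshActor in GrabVolume, disables its physics and attaches it to the controller mesh; release reverses this.
; Each tick tilts two stick components from the VR pawn's movement axes.
; Tick also displays the CPP_CPUUtilization actor's X location as the CPU value.
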(event Custom|StickRotation
  (bind _vrpawnreference (Variables|Default|GetVRPawnReference))
  (Transformation|SetRelativeRotation (Variables|Default|GetStickRotation_LR) (Math|Rotator|MakeRotator 0.0 (* (Variables|/Game/VR/BP_VR_Pawn.BP_VR_Pawn_C|GetMoveRight _vrpawnreference) 45.0) 0.0) false false)
  (Transformation|SetRelativeRotation (Variables|Default|GetStickRotation_UD) (Math|Rotator|MakeRotator (* (Variables|/Game/VR/BP_VR_Pawn.BP_VR_Pawn_C|GetMoveForward _vrpawnreference) 45.0) 0.0 0.0) false false))

(event EventBeginPlay
  (bind _asbp_vr_pawn (Utilities|Casting|CastToBP_VR_PawnClass "/Game/VR/BP_VR_Pawn.BP_VR_Pawn_C"))
  (bind _outactors (Actor|GetAllActorsOfClass _asbp_vr_pawn))
  (Variables|Default|SetVRPawnReference (Utilities|Array|Get(acopy) _outactors))
  (bind _ascpp_cpuutilization (Utilities|Casting|CastToCPP_CPUUtilizationClass "/Script/Intel_RCRaceland.CPP_CPUUtilization"))
  (bind _outactors_2 (Actor|GetAllActorsOfClass _ascpp_cpuutilization))
  (Variables|Default|SetCPPReference (Utilities|Array|Get(acopy) _outactors_2)))

(event EventTick
  (params (DeltaSeconds :type Float%20%28single-precision%29))
  (Utilities|FlowControl|Sequence
    (:then_0
      (Rendering|Components|TextRender|SetText (Variables|Default|GetText_FPS) (Utilities|Text|ToText(String) (Utilities|String|Append "CPU : " (Utilities|String|ToString(Text) (Utilities|Text|ToText(Float) (.x (Transformation|GetActorLocation (Variables|Default|GetCPPReference))) "HalfToEven" true 1 324 0 0))))))
    (:then_1
      (CallFunction|StickRotation))))

(fn ConstructionScript
  (Variables|/Script/HeadMountedDisplay.MotionControllerComponent|SetHand (Variables|Default|GetMotionController) (Variables|Default|GetHand)))

(fn GetMeshinRange
  (bind _grabvolume (Variables|Default|GetGrabVolume))
  (bind _returnvalue (Transformation|GetWorldLocation _grabvolume))
  (for _array_element (Collision|GetOverlappingActors _grabvolume "/Script/Engine.StaticMeshActor" :!class /Script/Engine.PrimitiveComponent)
    (bind _asstatic_mesh_actor (Utilities|Casting|CastToStaticMeshActor _array_element))
    (if (Physics|IsSimulatingPhysics (Variables|/Script/Engine.StaticMeshActor|GetStaticMeshComponent _asstatic_mesh_actor) "None")
      (if (< (Math|Vector|VectorLength (- (.OutPointOnBody (Collision|GetClosestPointonCollision (Variables|/Script/Engine.StaticMeshActor|GetStaticMeshComponent _asstatic_mesh_actor) _returnvalue "None")) _returnvalue)) (LocalVariables|GetNearOverlapDistance))
        (LocalVariables|SetNearOverlapMesh _asstatic_mesh_actor)
        (LocalVariables|SetNearOverlapDistance (Math|Vector|VectorLength (- (.OutPointOnBody (Collision|GetClosestPointonCollision (Variables|/Script/Engine.StaticMeshActor|GetStaticMeshComponent _asstatic_mesh_actor) _returnvalue "None")) _returnvalue))))))
  (return (LocalVariables|GetNearOverlapMesh)))

(fn ReleaseActor
  (Variables|Default|SetWantsToGrip? false)
  (Utilities|IsValid (Variables|Default|GetAttachedActor)
    (:Is%20Valid
      (Transformation|DetachFromActor (Variables|Default|GetAttachedActor) "KeepWorld" "KeepWorld" "KeepWorld")
      (Physics|SetSimulatePhysics (Variables|/Script/Engine.StaticMeshActor|GetStaticMeshComponent (Variables|Default|GetAttachedActor)) true)
      (Variables|Default|SetAttachedActor 0))))

(fn GrabActor
  (Variables|Default|SetWantsToGrip? true)
  (bind _nearestmesh (CallFunction|GetMeshinRange))
  (Utilities|IsValid _nearestmesh
    (:Is%20Valid
      (Variables|Default|SetAttachedActor _nearestmesh)
      (Physics|SetSimulatePhysics (Variables|/Script/Engine.StaticMeshActor|GetStaticMeshComponent _nearestmesh) false)
      (Transformation|AttachComponentToComponent _nearestmesh (Variables|Default|GetControllerMesh) "None" "KeepWorld" "KeepWorld" "KeepWorld" false))))
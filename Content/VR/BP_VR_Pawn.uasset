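; VR pawn that drives a vehicle already placed in the level using motion controllers.
; BeginPlay enables stereo with floor tracking, spawns left and right motion controllers on VRRoot with hand-specific text and stick visuals, and caches the first BPP_BaseVehicle found.
; Left thumbstick Y and right thumbstick X pass through a response curve into vehicle movement.
; Input actions handle handbrake and vehicle reset, and Escape exits.
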(event EventBeginPlay
  (bind _returnvalue (Math|Transform|MakeTransform "0, 0, 0" "0, 0,0.000000"))
  (bind _self self)
  (bind _vrroot (Variables|Default|GetVRRoot))
  (Development|ExecuteConsoleCommand "Stereo On")
  (Development|ExecuteConsoleCommand "r.ScreenPercentage 100")
  (Utilities|FlowControl|Sequence
    (:then_0
      (Class|HeadMountedDisplayFunctionLibrary|SetTrackingOrigin "Floor")
      (Components|Activation|SetActive (Variables|Default|GetCamera) true true))
    (:then_1
      (Utilities|FlowControl|Sequence
        (:then_0
          (bind _returnvalue_2 (Game|SpawnActorfromClass "/Game/VR/BP_MotionContoller.BP_MotionContoller_C" _returnvalue "AlwaysSpawn" _self "Left" 0))
          (bind _output_get (Variables|Default|SetLeftController _returnvalue_2))
          (Transformation|AttachComponentToComponent _output_get _vrroot "None" "SnapToTarget" "SnapToTarget" "KeepWorld" false)
          (Rendering|SetVisibility (Variables|/Game/VR/BP_MotionContoller.BP_MotionContoller_C|GetText_VehicleReset (Variables|Default|GetLeftController)) true true)
          (Development|SetHiddeninGame (Variables|/Game/VR/BP_MotionContoller.BP_MotionContoller_C|GetStickRoot_Left (Variables|Default|GetLeftController)) false true))
        (:then_1
          (bind _returnvalue_3 (Game|SpawnActorfromClass "/Game/VR/BP_MotionContoller.BP_MotionContoller_C" _returnvalue "AlwaysSpawn" _self "Right" 0))
          (bind _output_get_2 (Variables|Default|SetRightController _returnvalue_3))
          (Transformation|AttachComponentToComponent _output_get_2 _vrroot "None" "SnapToTarget" "SnapToTarget" "KeepWorld" false)
          (Rendering|SetVisibility (Variables|/Game/VR/BP_MotionContoller.BP_MotionContoller_C|GetText_FPS (Variables|Default|GetRightController)) true true)
          (Development|SetHiddeninGame (Variables|/Game/VR/BP_MotionContoller.BP_MotionContoller_C|GetStickRoot_Right (Variables|Default|GetRightController)) false true))))
    (:then_2
      (bind _asbpp_base_vehicle (Utilities|Casting|CastToBPP_BaseVehicleClass "/Game/Vehicles/BPP_BaseVehicle.BPP_BaseVehicle_C"))
      (bind _outactors (Actor|GetAllActorsOfClass _asbpp_base_vehicle))
      (Variables|Default|SetVehicleReference (Utilities|Array|Get(acopy) _outactors)))))

(event Input|ActionEvents|InputActionHandBrake
  (params (Key :type Key%20Structure :default "AnyKey"))
  (bind _vehiclereference (Variables|Default|GetVehicleReference))
  (bind _vehiclemovement (Variables|/Script/Engine.WheeledVehicle|GetVehicleMovement _vehiclereference))
  (:Pressed
    (Class|WheeledVehicleMovementComponent|SetHandbrakeInput _vehiclemovement true))
  (:Released
    (Class|WheeledVehicleMovementComponent|SetHandbrakeInput _vehiclemovement false)))

(event Input|ActionEvents|InputActionResetVehicle
  (params (Key :type Key%20Structure :default "AnyKey"))
  (:Pressed
    (Default|ResetVehicle (Variables|Default|GetVehicleReference))))

(event Input|KeyboardEvents|MotionControllerLeftThumbstickY
  (params (AxisValue :type Float%20%28single-precision%29))
  (bind _output_get (Variables|Default|SetMoveForward (Math|Curves|GetFloatValue (Variables|Default|GetVR_ControllerCurve) (* AxisValue -1.0))))
  (Default|SetMoveForward (Variables|Default|GetVehicleReference) _output_get))

(event Input|KeyboardEvents|MotionControllerRightThumbstickX
  (params (AxisValue :type Float%20%28single-precision%29))
  (bind _output_get (Variables|Default|SetMoveRight (Math|Curves|GetFloatValue (Variables|Default|GetVR_ControllerCurve) AxisValue)))
  (Default|SetMoveRight (Variables|Default|GetVehicleReference) _output_get))

(event Input|KeyboardEvents|Escape
  (params (Key :type Key%20Structure :default "AnyKey"))
  (:Pressed
    (Development|ExecuteConsoleCommand "Exit")))

(fn ConstructionScript)
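; BPC_RoomVRVehicle is a child vehicle Blueprint, apparently for a VR room, that keeps its UI facing the player.
; Each Tick calls the parent with zero delta time, then rotates UIPivot in world space along the look-at direction from the actor's location to the camera.
; BeginPlay's parent call is disabled, overlap is empty, and the construction script only calls the parent.
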(event EventBeginPlay
  (|CallParentFunction))

(event Collision|EventActorBeginOverlap
  (params (OtherActor :type Actor%20Object%20Reference)))

(event EventTick
  (params (DeltaSeconds :type Float%20%28single-precision%29))
  (|CallParentFunction 0.0)
  (Transformation|SetWorldRotation (Variables|Default|GetUI_Pivot) (Math|Rotator|FindLookatRotation (Transformation|GetActorLocation) (Camera|GetCameraLocation (Game|GetPlayerCameraManager 0))) false false))

(fn ConstructionScript
  (|CallParentFunction))
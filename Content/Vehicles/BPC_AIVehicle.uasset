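; BPC_AIVehicle is a self-driving vehicle Blueprint that holds a constant partial throttle and sets steering every tick, with R bound to reset the vehicle.
; Tick calls the parent, then SteerByWire feeds SteeringCalculation into the movement component's steering input.
; SteeringCalculation contains look-at math mapping yaw error toward a Steering target to a steering range, but that math is unconnected.
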(event Custom|SteerByWire
  (Class|WheeledVehicleMovementComponent|SetSteeringInput (Variables|Default|GetVehicleMovement) (Utilities|SteeringCalculation)))

(event EventTick
  (params (DeltaSeconds :type Float%20%28single-precision%29))
  (|CallParentFunction 0.0)
  (CallFunction|SteerbyWire)
  (Class|WheeledVehicleMovementComponent|SetThrottleInput (Variables|Default|GetVehicleMovement) 0.5))

(event Input|KeyboardEvents|R
  (params (Key :type Key%20Structure))
  (:Pressed
    (CallFunction|ResetVehicle)))

(fn ConstructionScript
  (|CallParentFunction))
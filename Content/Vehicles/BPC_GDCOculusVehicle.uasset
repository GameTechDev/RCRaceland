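; VR vehicle Blueprint, apparently for a GDC Oculus demo, extending a parent class with stereo rendering and debug inputs.
; BeginPlay turns stereo on via console command, while keyboard or gamepad buttons exit the game or toggle cloth optimization on every BP_FlagString actor as a test.
; SetVRSettings raises screen percentage when an HMD is enabled but is not called here, and a world-to-meters node is left unwired.
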(event EventBeginPlay
  (|CallParentFunction)
  (Development|ExecuteConsoleCommand "Stereo On"))

(event Collision|EventActorBeginOverlap
  (params (OtherActor :type Actor%20Object%20Reference)))

(event EventTick
  (params (DeltaSeconds :type Float%20%28single-precision%29))
  (|CallParentFunction DeltaSeconds))

(event Input|KeyboardEvents|O
  (params (Key :type Key%20Structure))
  (:Pressed
    (Tests|TESTFlagOptimizationSwitch)))

(event Input|GamepadEvents|GamepadSpecialLeft
  (params (Key :type Key%20Structure))
  (:Pressed
    (Tests|TESTFlagOptimizationSwitch)))

(event Input|KeyboardEvents|Escape
  (params (Key :type Key%20Structure))
  (:Pressed
    (Development|ExecuteConsoleCommand "Exit")))

(event Input|GamepadEvents|GamepadSpecialRight
  (params (Key :type Key%20Structure))
  (:Pressed
    (Development|ExecuteConsoleCommand "Exit")))

(fn ConstructionScript
  (|CallParentFunction))

(fn TESTFlagOptimizationSwitch
  (bind _asbp_flag_string (Utilities|Casting|CastToBP_FlagStringClass "/Game/FlagStrings/BP_FlagString.BP_FlagString_C"))
  (bind _outactors (Actor|GetAllActorsOfClass _asbp_flag_string))
  (for _array_element _outactors
    (Variables|/Game/FlagStrings/BP_FlagString.BP_FlagString_C|SetOptimizeCloth? _array_element (not (Variables|/Game/FlagStrings/BP_FlagString.BP_FlagString_C|GetOptimizeCloth? _array_element)))))

(fn SetVRSettings
  (if (Class|HeadMountedDisplayFunctionLibrary|IsHeadMountedDisplayEnabled)
    (Development|ExecuteConsoleCommand "r.screenpercentage 150")
    (Development|ExecuteConsoleCommand "Stereo On")))
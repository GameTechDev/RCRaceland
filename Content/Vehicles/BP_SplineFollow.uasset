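; BP_SplineFollow is a Blueprint that feeds a spline-following target to a vehicle.
; Each Tick, it projects a look-ahead point in front of the vehicle and finds the closest world-space location on the spline.
; That location is written to the vehicle's Steering variable and also positions a sphere at the target.
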(event EventTick
  (params (DeltaSeconds :type Float%20%28single-precision%29))
  (bind _spline (Variables|Default|GetSpline))
  (bind _vehicle (Variables|Default|GetVehicle))
  (bind _returnvalue (Transformation|GetActorLocation _vehicle))
  (bind _returnvalue_2 (Transformation|GetActorForwardVector _vehicle))
  (bind _returnvalue_3 (* _returnvalue_2 7.5e+02))
  (bind _returnvalue_4 (+ _returnvalue _returnvalue_3))
  (bind _returnvalue_5 (Spline|FindLocationClosesttoWorldLocation _spline _returnvalue_4 "World"))
  (Variables|/Game/Vehicles/BPC_FirstThirdPersonVehicleWithAI.BPC_FirstThirdPersonVehicleWithAI_C|SetSteering (Variables|Default|GetVehicle) _returnvalue_5)
  (Transformation|SetWorldLocation (Variables|Default|GetSphere) _returnvalue_5 false false))

(fn ConstructionScript)
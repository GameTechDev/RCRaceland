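; Configurable flag string prop strung between two poles, with optional pole accessories, top flags and cloth physics.
; The construction script builds the string from five-flag and single-flag skeletal mesh sections between eye-hooks, moving the second pole to its end.
; CreatePole dresses each pole from mesh table selections.
; With OptimizeCloth on, Tick raises flag minimum LOD to switch off cloth simulation while the actor is not recently rendered.
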(event Custom|SwitchClothSim
  ;[1 1 1] Sets all cloth meshes on the actor to LOD 0 or 1; turning cloth simulation on and off.     Dev Comment: Not the most efficent method because it is called and changed every tick, but is good enough for the purposes of this sample.
  (if (Variables|Settings|GetOptimizeCloth?)
    (if (not (Class|Actor|WasRecentlyRendered 0.05))
      (Class|SkinnedMeshComponent|SetMinLOD (Variables|Default|GetFlagTop01) 1)
      (for _array_element (Variables|Default|GetFlags)
        (if (!= _array_element 0)
          (Class|SkinnedMeshComponent|SetMinLOD _array_element 1)))
      (else
        (Class|SkinnedMeshComponent|SetMinLOD (Variables|Default|GetFlagTop01) :!label _label)
        (for _array_element_2 (Variables|Default|GetFlags)
          (if (!= _array_element_2 0)
            (Class|SkinnedMeshComponent|SetMinLOD _array_element_2)))))
    (else
      (goto _label))))

(event EventTick
  (params (DeltaSeconds :type Float%20%28single-precision%29))
  (CallFunction|SwitchClothSim))

(fn ConstructionScript
  (bind _pole01 (Variables|Default|GetPole01))
  (bind _pole02 (Variables|Default|GetPole02))
  ;[1 1 1] Create the flag string out to the number of flags set.
  (if (not (> (Variables|Settings|GetNumberOfFlags) 0))
    _
    (else
      (CallFunction|CreateFlagString)))
  (Utilities|FlowControl|Sequence
    (:then_0
      ;[1 1 1] Creates the first pole, then set it's height. Also sets the height and rotation of the pole accessory, and the rotation of the top flag.
      (CallFunction|CreatePole (Variables|Default|GetPole01) (Math|Conversions|ToInteger(Byte) (Variables|Pole1Settings|GetPole01_MeshTable)) (Variables|Default|GetAccessory01) (Math|Conversions|ToInteger(Byte) (Variables|Pole1Settings|GetPole01_AccessoryTable)) (Variables|Pole1Settings|GetPole01_FlagTop) (Variables|Default|GetFlagTop01))
      (Transformation|SetRelativeLocation _pole01 (Math|Vector|MakeVector (.x (Variables|/Script/Engine.SceneComponent|GetRelativeLocation _pole01)) 0.0 (Variables|Pole1Settings|GetPole01_Height)) false false)
      (Transformation|SetRelativeTransform (Variables|Default|GetAccessory01) (Math|Transform|MakeTransform (Math|Vector|MakeVector 0.0 0.0 (Variables|Pole1Settings|GetAccessory01_Height)) (Math|Rotator|MakeRotator 0.0 0.0 (Variables|Pole1Settings|GetAccessory01_Rotation)) "1,1,1") false false)
      (Transformation|SetRelativeRotation (Variables|Default|GetFlagTop01) (Math|Rotator|MakeRotator 0.0 0.0 (Variables|Pole1Settings|GetFlagTop01_Rotation)) false false))
    (:then_1
      ;[1 1 1] Creates the second pole, then set it's height. Also sets the height and rotation of the pole accessory, and the rotation of the top flag.
      (CallFunction|CreatePole (Variables|Default|GetPole02) (Math|Conversions|ToInteger(Byte) (Variables|Pole2Settings|GetPole02_MeshTable)) (Variables|Default|GetAccessory02) (Math|Conversions|ToInteger(Byte) (Variables|Pole2Settings|GetPole02_AccessoryTable)) (Variables|Pole2Settings|GetPole02_FlagTop) (Variables|Default|GetFlagTop02))
      (Transformation|SetRelativeLocation _pole02 (Math|Vector|MakeVector (.x (Variables|/Script/Engine.SceneComponent|GetRelativeLocation _pole02)) 0.0 (Variables|Pole2Settings|GetPole02_Height)) false false)
      (Transformation|SetRelativeTransform (Variables|Default|GetAccessory02) (Math|Transform|MakeTransform (Math|Vector|MakeVector 0.0 0.0 (Variables|Pole2Settings|GetAccessory02_Height)) (Math|Rotator|MakeRotator 0.0 0.0 (Variables|Pole2Settings|GetAccessory02_Rotation)) "1,1,1") false false)
      (Transformation|SetRelativeRotation (Variables|Default|GetFlagTop02) (Math|Rotator|MakeRotator 0.0 0.0 (Variables|Pole2Settings|GetFlagTop02_Rotation)) false false))))

(fn CreatePole
  (params (Pole :type Static%20Mesh%20Component%20Object%20Reference) (PoleTable :type Integer) (Accessory :type Static%20Mesh%20Component%20Object%20Reference) (AccessoryTable :type Integer) (UseFlagTop :type Boolean) (FlagTop :type Skeletal%20Mesh%20Component%20Object%20Reference))
  ;[1 1 1] Sets the pole based on the pole table. If the 4th option (none) is selected, end.
  (Components|StaticMesh|SetStaticMesh Pole (Utilities|Array|Get(acopy) (Variables|Default|GetPole_StaticMesh) PoleTable))
  (if (< PoleTable 3)
    ;[1 1 1] Set the accessory based on the accessory table.
    (Components|StaticMesh|SetStaticMesh Accessory (Utilities|Array|Get(acopy) (Variables|Default|GetAccessory_StaticMesh) AccessoryTable))
    ;[1 1 1] If the small pole and beam accessory are selected together, set mesh to none.
    (if (not (and (== PoleTable 0) (== AccessoryTable 2)))
      _
      (else
        (Components|StaticMesh|SetStaticMesh Accessory 0)))
    ;[1 1 1] If using flag top, set the skeletal mesh, and its height based on the pole selected.
    (if UseFlagTop
      (Class|SkinnedMeshComponent|SetSkeletalMesh FlagTop "/Game/FlagStrings/Models/SM_FlagString_TopFlag.SM_FlagString_TopFlag" true)
      (Transformation|SetRelativeLocation FlagTop (Utilities|Select :Index PoleTable :Option%200 "0,-5.000000,92.000000" :Option%201 "0.000000,-5.000000,146.000000" :Option%202 "0.000000,-5.000000,198.000000") false false)
      ;[1 1 1] If not using cloth physics, set the top flag's flag texture to the normal mapped flag texture.
      (bind _output_get (Variables|/Script/Engine.SkeletalMeshComponent|SetbDisableClothSimulation FlagTop (not (Variables|Settings|GetUseClothPhysics?))))
      (if _output_get
        (Rendering|Material|SetMaterial FlagTop 1 0)))))

(fn CreateFlagString
  (bind _numberofflags (Variables|Settings|GetNumberOfFlags))
  (bind _returnvalue (Math|Conversions|ToFloat(Integer) _numberofflags))
  (bind (_remainder _returnvalue_2) (Math|Float|Division(WholeandRemainder) _returnvalue 5.0))
  (Utilities|Array|Clear (Variables|Default|GetFlags))
  ;[1 1 1] Set the position of the first eye-hook.
  (AddComponent|AddStaticMeshComponent false (Math|Transform|MakeTransform (Math|Vector|MakeVector 7.0 0.0 (Variables|Settings|GetFlagString_Height)) "0, 0,0.000000" "1,1,1"))
  (for _index (range 1 _returnvalue_2)
    ;[1 1 1] Creates the number of 5 flags sections, and spaces them out using an offset.
    (bind _returnvalue_3 (AddComponent|AddSkeletalMeshComponent false (Math|Transform|MakeTransform (Math|Vector|MakeVector (+ (* (- _index 1) (LocalVariables|Get5FlagOffset)) 2e+01) 0.0 (Variables|Settings|GetFlagString_Height)) "0, 0,0.000000" "1,1.000000,1")))
    ;[1 1 1] Sets each sections cloth physics variable.
    (Variables|/Script/Engine.SkeletalMeshComponent|SetbDisableClothSimulation _returnvalue_3 (not (Variables|Settings|GetUseClothPhysics?)))
    (Utilities|Array|Add (Variables|Default|GetFlags) _returnvalue_3))
  (for _index_2 (range 1 (Math|Float|Truncate _remainder))
    ;[1 1 1] Creates the number of single flag sections, and spaces them out using an offset.
    (bind _returnvalue_4 (AddComponent|AddSkeletalMeshComponent false (Math|Transform|MakeTransform (Math|Vector|MakeVector (+ (+ (* (- _index 1) (LocalVariables|Get5FlagOffset)) -15.0) (* _index_2 (LocalVariables|Get1FlagOffset))) 0.0 (Variables|Settings|GetFlagString_Height)) "0, 0, 0" "1,1.000000,1.000000")))
    (Utilities|Array|Add (Variables|Default|GetFlags) _returnvalue_4))
  ;[1 1 1] Creates the second eye-hook at the end of the string.
  (AddComponent|AddStaticMeshComponent false (Math|Transform|MakeTransform (Math|Vector|MakeVector (+ (+ (* (- _index 1) (LocalVariables|Get5FlagOffset)) (* _index_2 (LocalVariables|Get1FlagOffset))) -3.0) 0.0 (Variables|Settings|GetFlagString_Height)) "0,180.000000, 0" "1,1,1"))
  ;[1 1 1] Places the second pole at the end of the flag string.
  (Transformation|SetRelativeLocation (Variables|Default|GetPole02) (Math|Vector|MakeVector (+ (+ (* (- _index 1) (LocalVariables|Get5FlagOffset)) (* _index_2 (LocalVariables|Get1FlagOffset))) 4.0) 0.0 0.0) false false))
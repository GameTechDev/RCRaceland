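; BP_PillarDM is a destructible pillar actor that replaces its destructible component with a new one after each fracture.
; On fracture, collision drops to physics-only, then switches off after a delay, and a second delay precedes destroying the component.
; AddNewDM then adds a replacement, passing the actor transform saved at BeginPlay as its relative transform.
; It binds the replacement's fracture event to OnFracture, which repeats the sequence indefinitely.
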(event OnComponentFracture(DestructibleComponent)
  (params (HitPoint :type Vector%20%28by%20ref%29 :default "0, 0, 0") (HitDirection :type Vector%20%28by%20ref%29 :default "0, 0, 0"))
  (Collision|SetCollisionEnabled (Variables|Default|GetDestructibleComponent) "PhysicsOnly")
  (Utilities|FlowControl|Delay 5.0)
  (Collision|SetCollisionEnabled (Variables|Default|GetDestructibleComponent) "NoCollision")
  (Utilities|FlowControl|Delay 3.0)
  (Components|DestroyComponent (Variables|Default|GetDestructibleComponent))
  (CallFunction|AddNewDM))

(event Custom|AddNewDM
  (bind _returnvalue (AddComponent|AddDestructibleComponent false (Variables|Default|GetStartingTransform)))
  (bind _output_get (Variables|Default|SetDMReference _returnvalue))
  (EventDispatchers|BindEventtoOnComponentFracture _output_get (delegate Custom|OnFracture)))

(event Custom|OnFracture
  (params (HitPoint :type Vector%20%28by%20ref%29) (HitDirection :type Vector%20%28by%20ref%29))
  (Collision|SetCollisionEnabled (Variables|Default|GetDMReference) "PhysicsOnly")
  (Utilities|FlowControl|Delay 5.0)
  (Collision|SetCollisionEnabled (Variables|Default|GetDMReference) "NoCollision")
  (Utilities|FlowControl|Delay 3.0)
  (Components|DestroyComponent (Variables|Default|GetDMReference))
  (CallFunction|AddNewDM))

(event EventBeginPlay
  (Variables|Default|SetStartingTransform (Transformation|GetActorTransform))
  (Variables|Default|SetDMReference (Variables|Default|GetDestructibleComponent)))

(fn ConstructionScript)